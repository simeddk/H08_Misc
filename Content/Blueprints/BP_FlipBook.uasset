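; BP_FlipBook is an actor that plays named Paper2D flipbook animations from a FlipBooks map.
; SetFlipBook swaps the component's flipbook by name and returns its duration.
; On BeginPlay it plays "Start", and on actor overlap "Hitted", using a RetriggerableDelay of that duration before switching to "Idle".
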(event `self.ReceiveBeginPlay`
  (bind _duration (`self.SetFlipBook` "Start"))
  (`KismetSystemLibrary.RetriggerableDelay` _duration)
  (`self.SetFlipBook` "Idle"))

(event `self.ReceiveActorBeginOverlap`
  (params (OtherActor :type "Actor Object Reference"))
  (bind _duration (`self.SetFlipBook` "Hitted"))
  (`KismetSystemLibrary.RetriggerableDelay` _duration)
  (`self.SetFlipBook` "Idle"))

(fn `SetFlipBook`
  (params (FlipBookName :type Name))
  (returns (Duration :type "Float (double-precision)"))
  (bind _value (`BlueprintMapLibrary.Map_Find` (`self.FlipBooks`) FlipBookName))
  (`PaperFlipbookComponent.SetFlipbook` (`self.PaperFlipbook`) _value)
  (return (`PaperFlipbook.GetTotalDuration` _value)))

(fn `UserConstructionScript`)