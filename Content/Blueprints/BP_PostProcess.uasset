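; BP_PostProcess is an actor that changes its post-process settings while a Character overlaps it.
; Begin overlap casts the other actor to Character, then writes raised intensity and focal distance values into the PostProcess settings struct.
; End overlap applies the same Character filter and sets both values back to zero, switching instantly with no blending in the graph.
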(event `self.ReceiveActorBeginOverlap`
  (params (OtherActor :type "Actor Object Reference"))
  (bind _settings (`PostProcessComponent.Settings` (`self.PostProcess`)))
  (cast `Character` OtherActor)
  (setmembers `PostProcessSettings` :`StructRef` _settings :`BloomIntensity` 8.0)
  (setmembers `PostProcessSettings` :`StructRef` _settings :`DepthOfFieldFocalDistance` 15.0))

(event `self.ReceiveActorEndOverlap`
  (params (OtherActor :type "Actor Object Reference"))
  (bind _settings (`PostProcessComponent.Settings` (`self.PostProcess`)))
  (cast `Character` OtherActor)
  (setmembers `PostProcessSettings` :`StructRef` _settings :`BloomIntensity` 0.0)
  (setmembers `PostProcessSettings` :`StructRef` _settings :`DepthOfFieldFocalDistance` 0.0))

(fn `UserConstructionScript`)