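; BP_Beacon is a level-travel trigger that opens another level when a Character overlaps it.
; The actor's first tag names the destination level, and Travel acts only if the overlapping actor is a Character and a tag exists.
; Tick draws that tag as debug text at the beacon's location, using the same IsActorTagValid check.
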(event `self.ReceiveActorBeginOverlap`
  (params (OtherActor :type "Actor Object Reference"))
  (`self.Travel` OtherActor))

(event `self.ReceiveTick`
  (params (DeltaSeconds :type "Float (single-precision)"))
  (if (`self.IsActorTagValid`)
    (`KismetSystemLibrary.DrawDebugString` (`self.K2_GetActorLocation`) (`KismetStringLibrary.Conv_NameToString` (`|GetArrayItem` (`self.Tags`))) null)))

(fn `IsActorTagValid`
  (returns (ReturnValue :type Boolean))
  (return (> (`KismetArrayLibrary.Array_Length` (`self.Tags`)) 0)))

(fn `Travel`
  (params (Object :type "Object Object Reference"))
  (cast `Character` Object)
  (if (`self.IsActorTagValid`)
    (`GameplayStatics.OpenLevel` (`|GetArrayItem` (`self.Tags`)))))

(fn `UserConstructionScript`)