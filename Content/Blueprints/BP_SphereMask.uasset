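; BP_SphereMask is an overlap-triggered actor that switches a post-process effect on while a Character is inside it.
; The PostProcess component starts disabled in both the construction script and BeginPlay.
; Begin and end overlap events cast the other actor to Character, then enable or disable the component, without counting overlaps or limiting it to the local player.
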(event `self.ReceiveBeginPlay`
  (set `PostProcessComponent.bEnabled` false (`self.PostProcess`)))

(event `self.ReceiveActorBeginOverlap`
  (params (OtherActor :type "Actor Object Reference"))
  (cast `Character` OtherActor)
  (set `PostProcessComponent.bEnabled` true (`self.PostProcess`)))

(event `self.ReceiveActorEndOverlap`
  (params (OtherActor :type "Actor Object Reference"))
  (cast `Character` OtherActor)
  (set `PostProcessComponent.bEnabled` false (`self.PostProcess`)))

(fn `UserConstructionScript`
  (set `PostProcessComponent.bEnabled` false (`self.PostProcess`)))